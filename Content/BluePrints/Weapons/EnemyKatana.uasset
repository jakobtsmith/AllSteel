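; EnemyKatana is an enemy melee weapon that damages the player on contact.
; Its Box collision starts disabled at BeginPlay, and nothing in this Blueprint re-enables it.
; When the box overlaps a PlayerBP while Hit is false, it subtracts Damage from the player's Health and sets IsDead from whether Health is zero or below.
; Hit is only read here, never set.
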(event OnComponentBeginOverlap(Box)
  (params (OverlappedComponent :type Primitive%20Component%20Object%20Reference) (OtherActor :type Actor%20Object%20Reference) (OtherComp :type Primitive%20Component%20Object%20Reference) (OtherBodyIndex :type Integer) (bFromSweep :type Boolean) (SweepResult :type Hit%20Result%20Structure%20%28by%20ref%29))
  ;[1 1 1] Deal Damage to Player
  (if (not (Variables|Default|GetHit))
    (bind _asplayer_bp (Utilities|Casting|CastToPlayerBP OtherActor))
    (bind _output_get (Variables|/Game/BluePrints/Player/PlayerBP.PlayerBP_C|SetHealth _asplayer_bp (- (Variables|/Game/BluePrints/Player/PlayerBP.PlayerBP_C|GetHealth _asplayer_bp) (Variables|Default|GetDamage))))
    (Variables|/Game/BluePrints/Player/PlayerBP.PlayerBP_C|SetIsDead _asplayer_bp (<= _output_get 0.0))))

(event EventBeginPlay
  ;[1 1 1] Disable Box Collision Initially
  (Collision|SetCollisionEnabled (Variables|Default|GetBox) "NoCollision"))

(fn ConstructionScript)