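; Knife weapon that damages the player character through a Box hit volume, whose collision starts disabled at BeginPlay.
; On overlap with a PlayerBP, a Hit flag allows one strike and is not reset within this Blueprint.
; Damage is halved when the player's ReduceDamage is set and both forward vectors are under 90 degrees apart.
; It subtracts the damage from Health directly and sets IsDead at zero or below.
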(event OnComponentBeginOverlap(Box)
  (params (OverlappedComponent :type Primitive%20Component%20Object%20Reference) (OtherActor :type Actor%20Object%20Reference) (OtherComp :type Primitive%20Component%20Object%20Reference) (OtherBodyIndex :type Integer) (bFromSweep :type Boolean) (SweepResult :type Hit%20Result%20Structure%20%28by%20ref%29))
  ;[1 1 1] Deal Damage to PC
  (bind _asplayer_bp (Utilities|Casting|CastToPlayerBP OtherActor))
  (bind _output_get (Variables|Default|SetSamurai _asplayer_bp))
  (if (not (Variables|Default|GetHit))
    (Variables|Default|SetHit true)
    (if (and (Variables|/Game/BluePrints/Player/PlayerBP.PlayerBP_C|GetReduceDamage _output_get) (< (Class|KismetMathLibrary|DegAcos (Math|Vector|DotProduct (Transformation|GetActorForwardVector OtherActor) (Transformation|GetActorForwardVector))) 9e+01))
      (Variables|/Game/BluePrints/Player/PlayerBP.PlayerBP_C|SetDealtDamage (Variables|Default|GetSamurai) 0.05)
      (else
        (Variables|/Game/BluePrints/Player/PlayerBP.PlayerBP_C|SetDealtDamage (Variables|Default|GetSamurai) 0.1)))
    (bind _output_get_2 (Variables|/Game/BluePrints/Player/PlayerBP.PlayerBP_C|SetHealth (Variables|Default|GetSamurai) (- (Variables|/Game/BluePrints/Player/PlayerBP.PlayerBP_C|GetHealth (Variables|Default|GetSamurai)) (Variables|/Game/BluePrints/Player/PlayerBP.PlayerBP_C|GetDealtDamage (Variables|Default|GetSamurai)))))
    (if (<= _output_get_2 0.0)
      (Variables|/Game/BluePrints/Player/PlayerBP.PlayerBP_C|SetIsDead (Variables|Default|GetSamurai) true))))

(event EventBeginPlay
  ;[1 1 1] Turn Off Collision
  (Collision|SetCollisionEnabled (Variables|Default|GetBox) "NoCollision"))

(fn ConstructionScript)