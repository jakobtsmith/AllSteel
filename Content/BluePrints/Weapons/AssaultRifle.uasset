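; Assault rifle weapon Blueprint that spawns ARBullet actors from its barrel when shooting starts.
; StartShooting sets IsFiring and calls FireBullet once, while StopShooting only clears the flag, with no repeat-fire loop in these graphs.
; FireBullet spawns at BarrelRefPoint, aiming along the skeletal mesh's right vector with random roll, pitch and yaw offsets within Spread.
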(event Custom|StartShooting
  (Variables|Default|SetIsFiring true)
  (CallFunction|FireBullet))

(event Custom|StopShooting
  (Variables|Default|SetIsFiring false))

(fn ConstructionScript)

(fn FireBullet
  (bind _skeletalmesh (Variables|Default|GetSkeletalMesh))
  (bind _spread (Variables|Default|GetSpread))
  (bind _returnvalue (- 0.0 _spread))
  (bind _returnvalue_2 (Math|Vector|GetRightVector _skeletalmesh))
  (bind _returnvalue_3 (Math|Conversions|RotationFromXVector _returnvalue_2))
  (Game|SpawnActorfromClass "/Game/BluePrints/Weapons/Ammo/ARBullet.ARBullet_C" (Math|Transform|MakeTransform (Transformation|GetWorldLocation (Variables|Default|GetBarrel_RefPoint)) (Math|Rotator|MakeRotator (+ (.roll _returnvalue_3) (Math|Random|RandomFloatinRange _returnvalue (Variables|Default|GetSpread))) (+ (.pitch _returnvalue_3) (Math|Random|RandomFloatinRange _returnvalue (Variables|Default|GetSpread))) (+ (.yaw _returnvalue_3) (Math|Random|RandomFloatinRange _returnvalue (Variables|Default|GetSpread)))) "1,1,1") "Undefined" 0 0))