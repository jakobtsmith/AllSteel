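; Player katana weapon that damages NPCs, the boss and the enemy samurai on box overlap, with collision off at BeginPlay.
; The player's HitTargets list blocks repeat hits, while current attack data sets damage and demon gauge gain.
; The boss takes damage only when stunned, otherwise turning via timeline to knock the player back.
; It also handles enemy deaths, the samurai's low-health demon form and the end-game screen on boss death.
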(event OnComponentBeginOverlap(Box)
  (params (OverlappedComponent :type Primitive%20Component%20Object%20Reference) (OtherActor :type Actor%20Object%20Reference) (OtherComp :type Primitive%20Component%20Object%20Reference) (OtherBodyIndex :type Integer) (bFromSweep :type Boolean) (SweepResult :type Hit%20Result%20Structure%20%28by%20ref%29))
  (bind _returnvalue (Game|GetPlayerCharacter 0))
  (bind _returnvalue_2 (Game|GetPlayerController 0))
  ;[1 1 1] Deal Damage to Enemy NPCs
  (bind _asplayer_bp (Utilities|Casting|CastToPlayerBP (Game|GetPlayerCharacter 0)))
  (Variables|Default|SetSamurai _asplayer_bp)
  (Variables|Default|SetHitTarget OtherActor)
  (if (not (Utilities|Array|ContainsItem (Variables|/Game/BluePrints/Player/PlayerBP.PlayerBP_C|GetHitTargets (Variables|Default|GetSamurai)) (Variables|Default|GetHitTarget)))
    (Utilities|Array|Add (Variables|/Game/BluePrints/Player/PlayerBP.PlayerBP_C|GetHitTargets (Variables|Default|GetSamurai)) (Variables|Default|GetHitTarget))
    (bind _asnpc_parent (Utilities|Casting|CastToNPC_Parent OtherActor)
      (:then
        (Variables|Default|SetNPC _asnpc_parent)
        (Variables|/Game/BluePrints/Player/PlayerBP.PlayerBP_C|SetDemonGauge (Variables|Default|GetSamurai) (Math|Float|Clamp(Float) (+ (Variables|/Game/BluePrints/Player/PlayerBP.PlayerBP_C|GetDemonGauge (Variables|Default|GetSamurai)) (.demonamount (Utilities|Array|Get(acopy) (Variables|/Game/BluePrints/Player/PlayerBP.PlayerBP_C|GetAttacks (Variables|Default|GetSamurai)) (Math|Conversions|ToInteger(Byte) (Variables|/Game/BluePrints/Player/PlayerBP.PlayerBP_C|GetAttack%20Type (Variables|Default|GetSamurai))))))))
        (bind _output_get (Variables|/Game/BluePrints/NPCs/EnemyTypes/NPC_Parent.NPC_Parent_C|SetHealth (Variables|Default|GetNPC) (- (Variables|/Game/BluePrints/NPCs/EnemyTypes/NPC_Parent.NPC_Parent_C|GetHealth (Variables|Default|GetNPC)) (* (.damageamount (Utilities|Array|Get(acopy) (Variables|/Game/BluePrints/Player/PlayerBP.PlayerBP_C|GetAttacks (Variables|Default|GetSamurai)) (Math|Conversions|ToInteger(Byte) (Variables|/Game/BluePrints/Player/PlayerBP.PlayerBP_C|GetAttack%20Type (Variables|Default|GetSamurai))))) (Variables|/Game/BluePrints/Player/PlayerBP.PlayerBP_C|GetDamageMod (Variables|Default|GetSamurai))))))
        (if (<= _output_get 0.001)
          (bind _ashudbp (Utilities|Casting|CastToHUDBP (HUD|GetHUD (Game|GetPlayerController 0))))
          (bind _result (Math|Integer|DecrementInt (Variables|/Game/BluePrints/Player/HUDBP.HUDBP_C|GetNumEnemies _ashudbp))
            (:%20%20
              (Variables|/Game/BluePrints/Player/PlayerBP.PlayerBP_C|SetKilledEnemies (Variables|Default|GetSamurai) (<= _result 0))
              (Actor|DestroyActor (Variables|Default|GetHitTarget))))))
      (:CastFailed
        ;[1 1 1] Deal Damage to Boss
        (bind _asboss_bp (Utilities|Casting|CastToBossBP OtherActor)
          (:then
            (bind _output_get_2 (Variables|Default|SetBoss _asboss_bp))
            (if (Variables|/Game/BluePrints/NPCs/Boss/BossBP.BossBP_C|GetStunned _output_get_2)
              (Variables|/Game/BluePrints/Player/PlayerBP.PlayerBP_C|SetDemonGauge (Variables|Default|GetSamurai) (Math|Float|Clamp(Float) (+ (Variables|/Game/BluePrints/Player/PlayerBP.PlayerBP_C|GetDemonGauge (Variables|Default|GetSamurai)) (.demonamount (Utilities|Array|Get(acopy) (Variables|/Game/BluePrints/Player/PlayerBP.PlayerBP_C|GetAttacks (Variables|Default|GetSamurai)) (Math|Conversions|ToInteger(Byte) (Variables|/Game/BluePrints/Player/PlayerBP.PlayerBP_C|GetAttack%20Type (Variables|Default|GetSamurai))))))))
              (bind _output_get_3 (Variables|/Game/BluePrints/NPCs/Boss/BossBP.BossBP_C|SetHealth (Variables|Default|GetBoss) (- (Variables|/Game/BluePrints/NPCs/Boss/BossBP.BossBP_C|GetHealth (Variables|Default|GetBoss)) (* (.damageamount (Utilities|Array|Get(acopy) (Variables|/Game/BluePrints/Player/PlayerBP.PlayerBP_C|GetAttacks (Variables|Default|GetSamurai)) (Math|Conversions|ToInteger(Byte) (Variables|/Game/BluePrints/Player/PlayerBP.PlayerBP_C|GetAttack%20Type (Variables|Default|GetSamurai))))) (Variables|/Game/BluePrints/Player/PlayerBP.PlayerBP_C|GetDamageMod (Variables|Default|GetSamurai))))))
              (if (<= _output_get_3 0.001)
                (Variables|/Game/BluePrints/NPCs/Boss/BossBP.BossBP_C|SetIsDead (Variables|Default|GetBoss) true)
                (Components|Animation|PlayAnimation (Variables|/Script/Engine.Character|GetMesh (Variables|Default|GetBoss)) "/Game/Models/Animations/Boss/Death_Anim_mixamo_com.Death_Anim_mixamo_com" false)
                (Development|SetHiddeninGame (Variables|/Game/BluePrints/NPCs/Boss/BossBP.BossBP_C|GetPaperSprite (Variables|Default|GetBoss)) true false)
                (bind _returnvalue_3 (UserInterface|CreateWidget "/Game/BluePrints/Widgets/EndGame.EndGame_C"))
                (Input|SetInputModeUIOnly _returnvalue_2 _returnvalue_3 "DoNotLock")
                (UserInterface|Viewport|AddtoViewport _returnvalue_3 0)
                (Variables|/Script/Engine.PlayerController|SetbShowMouseCursor _returnvalue_2 true)
                (Pawn|Components|CharacterMovement|DisableMovement (Variables|/Script/Engine.Character|GetCharacterMovement (Game|GetPlayerCharacter 0))))
              (else
                (Variables|/Game/BluePrints/Weapons/MiniGun.MiniGun_C|SetFiring (Variables|/Game/BluePrints/NPCs/Boss/BossBP.BossBP_C|GetGun (Variables|Default|GetBoss)) false)
                (Variables|/Game/BluePrints/NPCs/Boss/BossBP.BossBP_C|SetWasStunned (Variables|Default|GetBoss) true)
                (Utilities|Time|ClearandInvalidateTimerbyHandle (Variables|/Game/BluePrints/NPCs/Boss/BossBP.BossBP_C|GetSetSightsTimer (Variables|Default|GetBoss)))
                (Utilities|Time|ClearandInvalidateTimerbyHandle (Variables|/Game/BluePrints/NPCs/Boss/BossBP.BossBP_C|GetFiringTimer (Variables|Default|GetBoss)))
                (Components|Animation|PlayAnimation (Variables|/Script/Engine.Character|GetMesh (Variables|Default|GetBoss)) "/Game/Models/Boss/Rifle_Punch_mixamo_com.Rifle_Punch_mixamo_com" false)
                (bind _turn (Timeline|Timeline_0 PlayFromStart)
                  (:Update
                    (Transformation|SetActorRotation (Variables|Default|GetBoss) (Math|Rotator|MakeRotator 0.0 0.0 (Math|Float|Lerp (.yaw (Transformation|GetActorRotation (Variables|Default|GetBoss))) (+ (.yaw (Math|Rotator|FindLookatRotation (Transformation|GetActorLocation (Variables|Default|GetBoss)) (Transformation|GetActorLocation (Game|GetPlayerCharacter 0)))) 12.0) _turn))))
                  (:Finished
                    (Character|LaunchCharacter _returnvalue (Math|Vector|MakeVector (.x (* (Math|Vector|Normalize (- (Transformation|GetWorldLocation (Variables|/Script/Engine.Character|GetCapsuleComponent _returnvalue)) (Transformation|GetWorldLocation (Variables|/Script/Engine.Character|GetCapsuleComponent (Variables|Default|GetBoss))))) 2e+03)) (.y (* (Math|Vector|Normalize (- (Transformation|GetWorldLocation (Variables|/Script/Engine.Character|GetCapsuleComponent _returnvalue)) (Transformation|GetWorldLocation (Variables|/Script/Engine.Character|GetCapsuleComponent (Variables|Default|GetBoss))))) 2e+03)) 0.0) false false)
                    (Variables|/Game/BluePrints/Player/PlayerBP.PlayerBP_C|SetHealth (Variables|Default|GetSamurai) (- (Variables|/Game/BluePrints/Player/PlayerBP.PlayerBP_C|GetHealth (Variables|Default|GetSamurai)) 0.1))
                    (Components|Animation|PlayAnimation (Variables|/Script/Engine.Character|GetMesh (Variables|Default|GetBoss)) "/Game/Models/Animations/Boss/Idle_Anim_mixamo_com.Idle_Anim_mixamo_com" false)
                    (Default|ReturntoPhase (Variables|Default|GetBoss)))))))
          (:CastFailed
            ;[1 1 1] Deal Damge to Enemy Samurai
            (bind _assamurai_enemy (Utilities|Casting|CastToSamuraiEnemy OtherActor))
            (Variables|Default|SetSamuraiEnemy _assamurai_enemy)
            (Variables|/Game/BluePrints/Player/PlayerBP.PlayerBP_C|SetDemonGauge (Variables|Default|GetSamurai) (Math|Float|Clamp(Float) (+ (Variables|/Game/BluePrints/Player/PlayerBP.PlayerBP_C|GetDemonGauge (Variables|Default|GetSamurai)) (.demonamount (Utilities|Array|Get(acopy) (Variables|/Game/BluePrints/Player/PlayerBP.PlayerBP_C|GetAttacks (Variables|Default|GetSamurai)) (Math|Conversions|ToInteger(Byte) (Variables|/Game/BluePrints/Player/PlayerBP.PlayerBP_C|GetAttack%20Type (Variables|Default|GetSamurai))))))))
            (bind _output_get_4 (Variables|/Game/BluePrints/NPCs/EnemyTypes/SamuraiEnemy.SamuraiEnemy_C|SetHealth (Variables|Default|GetSamuraiEnemy) (- (Variables|/Game/BluePrints/NPCs/EnemyTypes/SamuraiEnemy.SamuraiEnemy_C|GetHealth _assamurai_enemy) (* (.damageamount (Utilities|Array|Get(acopy) (Variables|/Game/BluePrints/Player/PlayerBP.PlayerBP_C|GetAttacks (Variables|Default|GetSamurai)) (Math|Conversions|ToInteger(Byte) (Variables|/Game/BluePrints/Player/PlayerBP.PlayerBP_C|GetAttack%20Type (Variables|Default|GetSamurai))))) (Variables|/Game/BluePrints/Player/PlayerBP.PlayerBP_C|GetDamageMod (Variables|Default|GetSamurai))))))
            (if (<= _output_get_4 0.001)
              (Variables|/Game/BluePrints/NPCs/EnemyTypes/SamuraiEnemy.SamuraiEnemy_C|SetIsDead (Variables|Default|GetSamuraiEnemy) true)
              (Variables|/Game/BluePrints/NPCs/EnemyTypes/SamuraiEnemy.SamuraiEnemy_C|SetStarted (Variables|Default|GetSamuraiEnemy) false)
              (Components|Movement|StopMovementImmediately (Variables|/Script/Engine.Character|GetCharacterMovement (Variables|Default|GetSamuraiEnemy)))
              (Utilities|FlowControl|Delay 1.0)
              (Development|SetHiddeninGame (Variables|/Game/BluePrints/NPCs/EnemyTypes/SamuraiEnemy.SamuraiEnemy_C|GetEnemyHealth (Variables|Default|GetSamuraiEnemy)) true false)
              (Components|Activation|Deactivate (Variables|/Game/BluePrints/NPCs/EnemyTypes/SamuraiEnemy.SamuraiEnemy_C|GetDemonParticle (Variables|Default|GetSamuraiEnemy)))
              (Components|Activation|Deactivate (Variables|/Game/BluePrints/NPCs/EnemyTypes/SamuraiEnemy.SamuraiEnemy_C|GetRightDemonEye (Variables|Default|GetSamuraiEnemy)))
              (Components|Activation|Deactivate (Variables|/Game/BluePrints/NPCs/EnemyTypes/SamuraiEnemy.SamuraiEnemy_C|GetLeftDemonEye (Variables|Default|GetSamuraiEnemy)))
              (Development|SetHiddeninGame (Variables|/Game/BluePrints/NPCs/EnemyTypes/SamuraiEnemy.SamuraiEnemy_C|GetPaperSprite (Variables|Default|GetSamuraiEnemy)) true false)
              (Default|CallKilledMiniBoss)
              (Variables|/Game/BluePrints/Player/PlayerBP.PlayerBP_C|SetKilledMiniboss (Variables|Default|GetSamurai) true)
              (elif (<= _output_get_4 1.0)
                (if (not (Variables|/Game/BluePrints/NPCs/EnemyTypes/SamuraiEnemy.SamuraiEnemy_C|GetDemon (Variables|Default|GetSamuraiEnemy)))
                  (Variables|/Game/BluePrints/NPCs/EnemyTypes/SamuraiEnemy.SamuraiEnemy_C|SetDemon (Variables|Default|GetSamuraiEnemy) true)
                  (Components|Activation|Activate (Variables|/Game/BluePrints/NPCs/EnemyTypes/SamuraiEnemy.SamuraiEnemy_C|GetDemonParticle (Variables|Default|GetSamuraiEnemy)) false)
                  (Components|Activation|Activate (Variables|/Game/BluePrints/NPCs/EnemyTypes/SamuraiEnemy.SamuraiEnemy_C|GetRightDemonEye (Variables|Default|GetSamuraiEnemy)) false)
                  (Components|Activation|Activate (Variables|/Game/BluePrints/NPCs/EnemyTypes/SamuraiEnemy.SamuraiEnemy_C|GetLeftDemonEye (Variables|Default|GetSamuraiEnemy)) false))))))))))

(event EventBeginPlay
  ;[1 1 1] Disable Box Collision Initially
  (Collision|SetCollisionEnabled (Variables|Default|GetBox) "NoCollision"))

(fn ConstructionScript)