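; MiniGun is a weapon Blueprint that spins while firing and shoots bullet actors from its barrel.
; Tick rotates SpinRef on local pitch at a frame-rate-independent speed while Firing is set.
; FireBullet plays the minigun sound and spawns a MiniGunBullet at BarrelRef, taking only roll and yaw from the FireLocation vector's rotation, with pitch left unwired.
; The file shows no caller for FireBullet and no setter for Firing.
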(event EventTick
  (params (DeltaSeconds :type Float%20%28single-precision%29))
  (if (Variables|Default|GetFiring)
    (Transformation|AddLocalRotation (Variables|Default|GetSpinRef) (* (Math|Rotator|MakeRotator 0.0 7.2e+02 0.0) DeltaSeconds) false false)))

(fn ConstructionScript)

(fn FireBullet
  (bind _firelocation (Variables|Default|GetFireLocation))
  (bind _barrelref (Variables|Default|GetBarrelRef))
  (bind _returnvalue (Math|Conversions|RotationFromXVector _firelocation))
  (bind _returnvalue_2 (Transformation|GetWorldLocation _barrelref))
  (Audio|PlaySoundatLocation "/Game/Sounds/MinigunMiddle.MinigunMiddle" _returnvalue_2 "0, 0, 0" 1.0 1.0 0.0 0 0 0)
  (Game|SpawnActorfromClass "/Game/BluePrints/Weapons/Ammo/MiniGunBullet.MiniGunBullet_C" (Math|Transform|MakeTransform _returnvalue_2 (Math|Rotator|MakeRotator (.roll _returnvalue) 0.0 (.yaw _returnvalue)) "1,1,1") "Undefined" 0 0))