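; Player HUD that draws shrine save prompts, save results and the current objective as screen text.
; Each DrawHUD reads PlayerBP flags to choose a keyboard or gamepad save prompt, or a success or failure message.
; Outside the MainMenu level, kill flags step the objective from remaining enemies to the courtyard traitor to the grove leader.
; Text position and scale derive from screen size.
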(event EventDrawHUD
  (params (SizeX :type Integer) (SizeY :type Integer))
  (bind _output_get (Variables|Default|SetSizeX SizeX))
  (Variables|Default|SetObjectiveX (* _output_get 0.85))
  (bind _output_get_2 (Variables|Default|SetSizeY SizeY))
  (Variables|Default|SetObjectiveY (* _output_get_2 0.25))
  (Variables|Default|SetDrawScale (* (Variables|Default|GetSizeX) 0.000781))
  (bind _asplayer_bp (Utilities|Casting|CastToPlayerBP (Game|GetPlayerCharacter 0)))
  (Variables|Default|SetPlayer _asplayer_bp)
  (if (Variables|/Game/BluePrints/Player/PlayerBP.PlayerBP_C|GetNearShrine _asplayer_bp)
    (if (Variables|/Game/BluePrints/Player/PlayerBP.PlayerBP_C|GetUsingKeyboard _asplayer_bp)
      (HUD|DrawText "Press E to save" "(R=1.000000,G=1.000000,B=1.000000,A=1.000000)" (* (Variables|Default|GetSizeX) 0.45) (* (Variables|Default|GetSizeY) 0.85) 0 (Variables|Default|GetDrawScale) false)
      (else
        (HUD|DrawText "Press X to save" "(R=1.000000,G=1.000000,B=1.000000,A=1.000000)" (* (Variables|Default|GetSizeX) 0.45) (* (Variables|Default|GetSizeY) 0.85) 0 (Variables|Default|GetDrawScale) false)))
    (elif (Variables|/Game/BluePrints/Player/PlayerBP.PlayerBP_C|GetSaveSuccess _asplayer_bp)
      (HUD|DrawText "Successfully saved!" "(R=1.000000,G=1.000000,B=1.000000,A=1.000000)" (* (Variables|Default|GetSizeX) 0.45) (* (Variables|Default|GetSizeY) 0.85) 0 (Variables|Default|GetDrawScale) false)
      (elif (Variables|/Game/BluePrints/Player/PlayerBP.PlayerBP_C|GetSaveFailure _asplayer_bp)
        (HUD|DrawText "Failed to save" "(R=1.000000,G=1.000000,B=1.000000,A=1.000000)" (* (Variables|Default|GetSizeX) 0.45) (* (Variables|Default|GetSizeY) 0.85) 0 (Variables|Default|GetDrawScale) false))))
  (bind _returnvalue (Game|GetCurrentLevelName true))
  (if (Utilities|Enum|NotEqual(Enum) _returnvalue "MainMenu")
    (if (Variables|/Game/BluePrints/Player/PlayerBP.PlayerBP_C|GetKilledEnemies (Variables|Default|GetPlayer))
      (if (Variables|/Game/BluePrints/Player/PlayerBP.PlayerBP_C|GetKilledMiniboss (Variables|Default|GetPlayer))
        (HUD|DrawText "Objective: Defeat the leader 
in the grove past the stone  
doors." "(R=1.000000,G=1.000000,B=1.000000,A=1.000000)" (Variables|Default|GetObjectiveX) (Variables|Default|GetObjectiveY) 0 (Variables|Default|GetDrawScale) false)
        (else
          (HUD|DrawText "Objective: Deal with the traitor 
in the courtyard." "(R=1.000000,G=1.000000,B=1.000000,A=1.000000)" (Variables|Default|GetObjectiveX) (Variables|Default|GetObjectiveY) 0 (Variables|Default|GetDrawScale) false)))
      (else
        (HUD|DrawText (Utilities|String|Append "Objective: Kill Invading Enemies.  
" (Utilities|String|ToString(Integer) (Variables|Default|GetNumEnemies)) " remaining") "(R=1.000000,G=1.000000,B=1.000000,A=1.000000)" (Variables|Default|GetObjectiveX) (Variables|Default|GetObjectiveY) 0 (Variables|Default|GetDrawScale) false)))))

(fn ConstructionScript)