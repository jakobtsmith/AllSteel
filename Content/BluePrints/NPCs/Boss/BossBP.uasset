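; Boss NPC that attacks the player with a child-actor minigun and shows its health widget once activated.
; Phase 1 loops a timer that turns it toward the player by timeline, fires a timed burst, then plays reloading.
; A stun halts both timers, then plays a recovery and melee swing that launches a nearby player before resuming the current phase.
; Phase 2 is a stub that only sets the phase number.
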(event Custom|SetSights
  (bind _gun (Variables|Default|GetGun))
  (bind _turn (Timeline|Timeline_0 PlayFromStart)
    (:Update
      (Transformation|SetActorRotation (Math|Rotator|MakeRotator 0.0 0.0 (Math|Float|Lerp (.yaw (Transformation|GetActorRotation)) (+ (.yaw (Math|Rotator|FindLookatRotation (Transformation|GetActorLocation) (Transformation|GetActorLocation (Game|GetPlayerCharacter 0)))) 12.0) _turn))))
    (:Finished
      (Variables|Default|SetDamageThisBurst 0.0)
      (Transformation|SetRelativeLocationAndRotation (Variables|Default|GetMiniGun) "-82.255371,-180.058502,-3.504017" "78.742645,179.613892,373.698334" false false)
      (Components|Animation|PlayAnimation (Variables|Character|GetMesh) "/Game/Models/Animations/Boss/Idle_Anim_mixamo_com.Idle_Anim_mixamo_com" true)
      (Audio|PlaySoundatLocation "/Game/Sounds/MinigunStart.MinigunStart" (Transformation|GetActorLocation (Variables|/Script/Engine.ChildActorComponent|GetChildActor (Variables|Default|GetMiniGun))) "0, 0, 0" 1.0 1.0 0.0 0 0 0)
      (Variables|/Game/BluePrints/Weapons/MiniGun.MiniGun_C|SetFireLocation _gun (Math|Vector|GetRightVector (Components|GetChildComponent (Variables|Default|GetMiniGun) 0)))
      (Variables|/Game/BluePrints/Weapons/MiniGun.MiniGun_C|SetFiring _gun true)
      (bind _returnvalue (Utilities|Time|SetTimerbyFunctionName (Variables|Default|GetGun) "FireBullet" (Variables|Default|GetFireRate) true))
      (Variables|Default|SetFiringTimer _returnvalue)
      (Utilities|FlowControl|Delay 5.0)
      (Utilities|Time|ClearandInvalidateTimerbyHandle (Variables|Default|GetFiringTimer))
      (if (Variables|Default|GetWasStunned)
        (Variables|Default|SetWasStunned false)
        (else
          (Audio|PlaySoundatLocation "/Game/Sounds/MinigunEnd.MinigunEnd" (Transformation|GetActorLocation (Variables|/Script/Engine.ChildActorComponent|GetChildActor (Variables|Default|GetMiniGun))) "0, 0, 0" 1.0 1.0 0.0 0 0 0)
          (Variables|/Game/BluePrints/Weapons/MiniGun.MiniGun_C|SetFiring (Variables|Default|GetGun) false)
          (Transformation|SetRelativeLocationAndRotation (Variables|Default|GetMiniGun) "-21.883961,-208.867523,55.618744" "69.624962,132.813126,303.359558" false false)
          (Components|Animation|PlayAnimation (Variables|Character|GetMesh) "/Game/Models/Animations/Boss/Reloading_Anim_mixamo_com.Reloading_Anim_mixamo_com" false))))))

(event Custom|Phase1
  (Variables|Default|SetStunned false)
  (Variables|Default|SetCurrentPhase 1)
  (bind _returnvalue (Utilities|Time|SetTimerbyEvent (delegate Custom|SetSights) 8.3 true))
  (Variables|Default|SetSetSightsTimer _returnvalue)
  (CallFunction|SetSights))

(event Custom|Activated
  (Development|SetHiddeninGame (Variables|Default|GetHealthDisplay) false false)
  (CallFunction|Phase1))

(event Custom|BossStunned
  (bind _returnvalue (Game|GetPlayerCharacter 0))
  (bind _capsulecomponent (Variables|Collision|GetCapsuleComponent))
  (bind _returnvalue_2 (Transformation|GetWorldLocation _capsulecomponent))
  (bind _capsulecomponent_2 (Variables|/Script/Engine.Character|GetCapsuleComponent _returnvalue))
  (bind _returnvalue_3 (Transformation|GetWorldLocation _capsulecomponent_2))
  (bind _returnvalue_4 (- _returnvalue_3 _returnvalue_2))
  (bind _returnvalue_5 (Math|Vector|Normalize _returnvalue_4))
  (bind _returnvalue_6 (* _returnvalue_5 1e+03))
  (Variables|/Game/BluePrints/Weapons/MiniGun.MiniGun_C|SetFiring (Variables|Default|GetGun) false)
  (Utilities|Time|ClearandInvalidateTimerbyHandle (Variables|Default|GetFiringTimer))
  (Utilities|Time|ClearandInvalidateTimerbyHandle (Variables|Default|GetSetSightsTimer))
  (Components|Animation|PlayAnimation (Variables|Character|GetMesh) "/Game/Models/Animations/Boss/Stunned_Anim_mixamo_com.Stunned_Anim_mixamo_com" false)
  (Utilities|FlowControl|Delay 2.133333)
  (if (not (Variables|Default|GetIsDead))
    (Components|Animation|PlayAnimation (Variables|Character|GetMesh) "/Game/Models/Animations/Boss/Getting_Up_Anim_mixamo_com.Getting_Up_Anim_mixamo_com" false)
    (Utilities|FlowControl|Delay 4.316)
    (if (not (Variables|Default|GetIsDead))
      (Components|Animation|PlayAnimation (Variables|Character|GetMesh) "/Game/Models/Boss/Sword_And_Shield_Slash_Anim_mixamo_com.Sword_And_Shield_Slash_Anim_mixamo_com" false)
      (Transformation|SetRelativeLocation (Variables|Character|GetMesh) (Math|Vector|MakeVector -2.6e+02 7e+01 -87.240997) false false)
      (Utilities|FlowControl|Delay 0.312)
      (if (not (Variables|Default|GetIsDead))
        (Audio|PlaySoundatLocation "/Game/Sounds/Upper_Cut-SoundBible_com-1272257235.Upper_Cut-SoundBible_com-1272257235" (Transformation|GetActorLocation (Variables|/Script/Engine.ChildActorComponent|GetChildActor (Variables|Default|GetMiniGun))) "0, 0, 0" 1.0 1.0 0.0 0 0 0)
        (if (<= (Math|Vector|Distance2D(Vector) (Math|Conversions|ToVector2D(Vector) _returnvalue_3) (Math|Conversions|ToVector2D(Vector) _returnvalue_2)) 3e+02)
          (Character|LaunchCharacter _returnvalue (Math|Vector|MakeVector (.x _returnvalue_6) (.y _returnvalue_6) 1e+03) false false))
        (Utilities|FlowControl|Delay 0.868)
        (if (not (Variables|Default|GetIsDead))
          (Components|Animation|PlayAnimation (Variables|Character|GetMesh) "/Game/Models/Animations/Boss/Idle_Anim_mixamo_com.Idle_Anim_mixamo_com" false)
          (Transformation|SetRelativeLocation (Variables|Character|GetMesh) (Math|Vector|MakeVector -2.316 -8.643 -87.240997) false false)
          (CallFunction|ReturntoPhase))))))

(event Custom|ReturnToPhase
  (switch int (Variables|Default|GetCurrentPhase)
    (:1
      (CallFunction|Phase1))
    (:2
      (CallFunction|Phase2))))

(event Custom|Phase2
  (Variables|Default|SetCurrentPhase 2))

(event EventBeginPlay
  (bind _healthdisplay (Variables|Default|GetHealthDisplay))
  (bind _papersprite (Variables|Default|GetPaperSprite))
  (bind _asmini_gun (Utilities|Casting|CastToMiniGun (Variables|/Script/Engine.ChildActorComponent|GetChildActor (Variables|Default|GetMiniGun))))
  (Variables|Default|SetGun _asmini_gun)
  (Actor|SetOwner (Components|GetOwner _papersprite) (Game|GetPlayerCharacter 0))
  (Class|PrimitiveComponent|SetOwnerNoSee _papersprite true)
  (bind _asboss_health (Utilities|Casting|CastToBossHealth (UserInterface|GetUserWidgetObject _healthdisplay)))
  (Variables|/Game/BluePrints/NPCs/Boss/BossHealth.BossHealth_C|SetOwner _asboss_health self)
  (Development|SetHiddeninGame _healthdisplay true false))

(fn ConstructionScript)