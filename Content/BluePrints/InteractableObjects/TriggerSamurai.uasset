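; A trigger volume that wakes a linked SamuraiEnemy and moves a door when the player first enters it.
; The one-shot box overlap calls the enemy's Activated and plays a timeline that lerps the door from its current transform toward EndTransform.
; A separate OpenDoor event plays a second timeline in reverse, lerping the door toward the start transform cached on BeginPlay.
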(event OnComponentBeginOverlap(Box)
  (params (OverlappedComponent :type Primitive%20Component%20Object%20Reference) (OtherActor :type Actor%20Object%20Reference) (OtherComp :type Primitive%20Component%20Object%20Reference) (OtherBodyIndex :type Integer) (bFromSweep :type Boolean) (SweepResult :type Hit%20Result%20Structure%20%28by%20ref%29))
  (bind _door (Variables|Default|GetDoor))
  (Utilities|Casting|CastToPlayerBP OtherActor)
  (if (not (Variables|Default|GetActivated))
    (Variables|Default|SetActivated true)
    (bind _assamurai_enemy (Utilities|Casting|CastToSamuraiEnemy (Variables|Default|GetSamuraiEnemy)))
    (Default|Activated _assamurai_enemy)
    (bind _newtrack_0 (Timeline|Timeline_0 PlayFromStart)
      (:Update
        (Transformation|SetActorTransform _door (Math|Transform|Lerp(Transform) (Transformation|GetActorTransform _door) (Variables|Default|GetEndTransform) _newtrack_0))))))

(event Custom|OpenDoor
  (bind _door (Variables|Default|GetDoor))
  (bind _newtrack_0 (Timeline|Timeline_1 ReverseFromEnd)
    (:Update
      (Transformation|SetActorTransform _door (Math|Transform|Lerp(Transform) (Transformation|GetActorTransform _door) (Variables|Default|GetStartTransform) _newtrack_0)))))

(event EventBeginPlay
  (Variables|Default|SetStartTransform (Transformation|GetActorTransform (Variables|Default|GetDoor))))

(fn ConstructionScript)