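; SaveShrine is a one-use interactable checkpoint that saves the game when the player presses E or gamepad face-left nearby.
; Box overlap toggles input and the player's NearShrine flag.
; Activation refills Spirit Emblems, then snapshots the level name, player, every NPC_Parent (including blackboard AI state) and all shrines into an AllSteelSave.
; An async write to the "ShrineSave" slot briefly flags success or failure on the player, re-arming the shrine on failure.
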(event OnComponentBeginOverlap(Box)
  (params (OverlappedComponent :type Primitive%20Component%20Object%20Reference) (OtherActor :type Actor%20Object%20Reference) (OtherComp :type Primitive%20Component%20Object%20Reference) (OtherBodyIndex :type Integer) (bFromSweep :type Boolean) (SweepResult :type Hit%20Result%20Structure%20%28by%20ref%29))
  (if (not (Variables|Default|GetUsed))
    (bind _asplayer_bp (Utilities|Casting|CastToPlayerBP OtherActor))
    (bind _output_get (Variables|Default|SetSamurai _asplayer_bp))
    (Variables|/Game/BluePrints/Player/PlayerBP.PlayerBP_C|SetNearShrine _output_get true)
    (Input|EnableInput (Game|GetPlayerController 0))))

(event OnComponentEndOverlap(Box)
  (params (OverlappedComponent :type Primitive%20Component%20Object%20Reference) (OtherActor :type Actor%20Object%20Reference) (OtherComp :type Primitive%20Component%20Object%20Reference) (OtherBodyIndex :type Integer))
  (bind _asplayer_bp (Utilities|Casting|CastToPlayerBP OtherActor))
  (Variables|/Game/BluePrints/Player/PlayerBP.PlayerBP_C|SetNearShrine _asplayer_bp false)
  (Input|DisableInput (Game|GetPlayerController 0)))

(event Input|KeyboardEvents|E
  (params (Key :type Key%20Structure :default "None"))
  (bind _samurai (Variables|Default|GetSamurai))
  (bind _samurai_2 (Variables|Default|GetSamurai))
  (:Pressed
    (if (not (Variables|Default|GetUsed))
      (Variables|Default|SetUsed true)
      (Variables|/Game/BluePrints/Player/PlayerBP.PlayerBP_C|SetSpiritEmblems (Variables|Default|GetSamurai) 3)
      (Utilities|Array|Clear (Variables|Default|GetActorList))
      (bind _returnvalue (SaveGame|CreateSaveGameObject "/Game/AllSteelSave.AllSteelSave_C"))
      (bind _output_get (Variables|Default|SetSaveData _returnvalue))
      (bind _returnvalue_2 (Game|GetCurrentLevelName true))
      (Variables|/Game/AllSteelSave.AllSteelSave_C|SetLevelName _output_get (Utilities|String|StringToName _returnvalue_2))
      (bind _outactors (Actor|GetAllActorsOfClass "/Game/BluePrints/NPCs/EnemyTypes/NPC_Parent.NPC_Parent_C"))
      (for _array_element _outactors
        (Utilities|Array|Add (Variables|/Game/AllSteelSave.AllSteelSave_C|GetEnemySaveData (Variables|Default|GetSaveData)) (Utilities|Struct|MakeEnemySaveData (Utilities|GetClass _array_element) (Transformation|GetActorLocation _array_element) (Transformation|GetActorScale3D _array_element) (Transformation|GetActorRotation _array_element) (Variables|/Game/BluePrints/NPCs/EnemyTypes/NPC_Parent.NPC_Parent_C|GetHealth _array_element) (Variables|/Game/BluePrints/NPCs/EnemyTypes/NPC_Parent.NPC_Parent_C|GetLeashDistance _array_element) (Variables|/Game/BluePrints/NPCs/EnemyTypes/NPC_Parent.NPC_Parent_C|GetAttackDistance _array_element) (Variables|/Game/BluePrints/NPCs/EnemyTypes/NPC_Parent.NPC_Parent_C|GetPatrolPath _array_element) (Class|BlackboardComponent|GetValueasInt (AI|GetBlackboard _array_element) (Utilities|Name|MakeLiteralName "PatrolPathIndex")) (Class|BlackboardComponent|GetValueasInt (AI|GetBlackboard _array_element) (Utilities|Name|MakeLiteralName "Direction")) (Utilities|Enum|ByteToEnumEEnemyState (Class|BlackboardComponent|GetValueasEnum (AI|GetBlackboard _array_element) (Utilities|Name|MakeLiteralName "EnemyState"))))))
      (bind _asplayer_bp (Utilities|Casting|CastToPlayerBP (Game|GetPlayerCharacter 0)))
      (Variables|/Game/AllSteelSave.AllSteelSave_C|SetPlayerSaveData (Variables|Default|GetSaveData) (Utilities|Struct|MakePlayerSaveData (Variables|/Game/BluePrints/Player/PlayerBP.PlayerBP_C|GetHealth _asplayer_bp) (Variables|/Game/BluePrints/Player/PlayerBP.PlayerBP_C|GetFatigue _asplayer_bp) (Variables|/Game/BluePrints/Player/PlayerBP.PlayerBP_C|GetDemonGauge _asplayer_bp) (Variables|/Game/BluePrints/Player/PlayerBP.PlayerBP_C|GetSpiritEmblems _asplayer_bp) (Transformation|GetActorLocation _asplayer_bp) (Transformation|GetActorScale3D _asplayer_bp) (Transformation|GetActorRotation _asplayer_bp) (Variables|/Game/BluePrints/Player/PlayerBP.PlayerBP_C|GetKilledMiniboss _asplayer_bp) (Variables|/Game/BluePrints/Player/PlayerBP.PlayerBP_C|GetKilledEnemies _asplayer_bp)))
      (bind _outactors_2 (Actor|GetAllActorsOfClass "SaveShrine_C"))
      (for _array_element_2 _outactors_2
        (Utilities|Array|Add (Variables|/Game/AllSteelSave.AllSteelSave_C|GetSaveShrineData (Variables|Default|GetSaveData)) (Utilities|Struct|MakeSaveShrineData (Transformation|GetActorTransform _array_element_2) (Variables|SaveShrine_C|GetUsed _array_element_2))))
      (bind _bsuccess (|AsyncSaveGametoSlot (Variables|Default|GetSaveData) "ShrineSave")
        (:Completed
          (if _bsuccess
            (Variables|Default|SetUsed true)
            (Variables|/Game/BluePrints/Player/PlayerBP.PlayerBP_C|SetNearShrine _samurai_2 false)
            (Variables|/Game/BluePrints/Player/PlayerBP.PlayerBP_C|SetSaveSuccess _samurai_2 true)
            (Variables|/Game/BluePrints/Player/PlayerBP.PlayerBP_C|SetSaveFailure _samurai_2 false)
            (Utilities|FlowControl|Delay 2.0)
            (Variables|/Game/BluePrints/Player/PlayerBP.PlayerBP_C|SetSaveSuccess _samurai_2 false)
            (Input|DisableInput (Game|GetPlayerController 0))
            (else
              (Variables|Default|SetUsed false)
              (Variables|/Game/BluePrints/Player/PlayerBP.PlayerBP_C|SetSaveSuccess _samurai false)
              (Variables|/Game/BluePrints/Player/PlayerBP.PlayerBP_C|SetSaveFailure _samurai true)
              (Utilities|FlowControl|Delay 2.0)
              (Variables|/Game/BluePrints/Player/PlayerBP.PlayerBP_C|SetSaveFailure _samurai false))))))))

(event Input|GamepadEvents|GamepadFaceButtonLeft
  (params (Key :type Key%20Structure :default "None"))
  (bind _samurai (Variables|Default|GetSamurai))
  (bind _samurai_2 (Variables|Default|GetSamurai))
  (:Pressed
    (if (not (Variables|Default|GetUsed))
      (Variables|Default|SetUsed true)
      (Variables|/Game/BluePrints/Player/PlayerBP.PlayerBP_C|SetSpiritEmblems (Variables|Default|GetSamurai) 3)
      (Utilities|Array|Clear (Variables|Default|GetActorList))
      (bind _returnvalue (SaveGame|CreateSaveGameObject "/Game/AllSteelSave.AllSteelSave_C"))
      (bind _output_get (Variables|Default|SetSaveData _returnvalue))
      (bind _returnvalue_2 (Game|GetCurrentLevelName true))
      (Variables|/Game/AllSteelSave.AllSteelSave_C|SetLevelName _output_get (Utilities|String|StringToName _returnvalue_2))
      (bind _outactors (Actor|GetAllActorsOfClass "/Game/BluePrints/NPCs/EnemyTypes/NPC_Parent.NPC_Parent_C"))
      (for _array_element _outactors
        (Utilities|Array|Add (Variables|/Game/AllSteelSave.AllSteelSave_C|GetEnemySaveData (Variables|Default|GetSaveData)) (Utilities|Struct|MakeEnemySaveData (Utilities|GetClass _array_element) (Transformation|GetActorLocation _array_element) (Transformation|GetActorScale3D _array_element) (Transformation|GetActorRotation _array_element) (Variables|/Game/BluePrints/NPCs/EnemyTypes/NPC_Parent.NPC_Parent_C|GetHealth _array_element) (Variables|/Game/BluePrints/NPCs/EnemyTypes/NPC_Parent.NPC_Parent_C|GetLeashDistance _array_element) (Variables|/Game/BluePrints/NPCs/EnemyTypes/NPC_Parent.NPC_Parent_C|GetAttackDistance _array_element) (Variables|/Game/BluePrints/NPCs/EnemyTypes/NPC_Parent.NPC_Parent_C|GetPatrolPath _array_element) (Class|BlackboardComponent|GetValueasInt (AI|GetBlackboard _array_element) (Utilities|Name|MakeLiteralName "PatrolPathIndex")) (Class|BlackboardComponent|GetValueasInt (AI|GetBlackboard _array_element) (Utilities|Name|MakeLiteralName "Direction")) (Utilities|Enum|ByteToEnumEEnemyState (Class|BlackboardComponent|GetValueasEnum (AI|GetBlackboard _array_element) (Utilities|Name|MakeLiteralName "EnemyState"))))))
      (bind _asplayer_bp (Utilities|Casting|CastToPlayerBP (Game|GetPlayerCharacter 0)))
      (Variables|/Game/AllSteelSave.AllSteelSave_C|SetPlayerSaveData (Variables|Default|GetSaveData) (Utilities|Struct|MakePlayerSaveData (Variables|/Game/BluePrints/Player/PlayerBP.PlayerBP_C|GetHealth _asplayer_bp) (Variables|/Game/BluePrints/Player/PlayerBP.PlayerBP_C|GetFatigue _asplayer_bp) (Variables|/Game/BluePrints/Player/PlayerBP.PlayerBP_C|GetDemonGauge _asplayer_bp) (Variables|/Game/BluePrints/Player/PlayerBP.PlayerBP_C|GetSpiritEmblems _asplayer_bp) (Transformation|GetActorLocation _asplayer_bp) (Transformation|GetActorScale3D _asplayer_bp) (Transformation|GetActorRotation _asplayer_bp) (Variables|/Game/BluePrints/Player/PlayerBP.PlayerBP_C|GetKilledMiniboss _asplayer_bp) (Variables|/Game/BluePrints/Player/PlayerBP.PlayerBP_C|GetKilledEnemies _asplayer_bp)))
      (bind _outactors_2 (Actor|GetAllActorsOfClass "SaveShrine_C"))
      (for _array_element_2 _outactors_2
        (Utilities|Array|Add (Variables|/Game/AllSteelSave.AllSteelSave_C|GetSaveShrineData (Variables|Default|GetSaveData)) (Utilities|Struct|MakeSaveShrineData (Transformation|GetActorTransform _array_element_2) (Variables|SaveShrine_C|GetUsed _array_element_2))))
      (bind _bsuccess (|AsyncSaveGametoSlot (Variables|Default|GetSaveData) "ShrineSave")
        (:Completed
          (if _bsuccess
            (Variables|Default|SetUsed true)
            (Variables|/Game/BluePrints/Player/PlayerBP.PlayerBP_C|SetNearShrine _samurai_2 false)
            (Variables|/Game/BluePrints/Player/PlayerBP.PlayerBP_C|SetSaveSuccess _samurai_2 true)
            (Variables|/Game/BluePrints/Player/PlayerBP.PlayerBP_C|SetSaveFailure _samurai_2 false)
            (Utilities|FlowControl|Delay 2.0)
            (Variables|/Game/BluePrints/Player/PlayerBP.PlayerBP_C|SetSaveSuccess _samurai_2 false)
            (Input|DisableInput (Game|GetPlayerController 0))
            (else
              (Variables|Default|SetUsed false)
              (Variables|/Game/BluePrints/Player/PlayerBP.PlayerBP_C|SetSaveSuccess _samurai false)
              (Variables|/Game/BluePrints/Player/PlayerBP.PlayerBP_C|SetSaveFailure _samurai true)
              (Utilities|FlowControl|Delay 2.0)
              (Variables|/Game/BluePrints/Player/PlayerBP.PlayerBP_C|SetSaveFailure _samurai false))))))))

(fn ConstructionScript)